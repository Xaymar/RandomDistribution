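; Swinging door actor that opens while pawns are inside its trigger box and closes when the last one leaves.
; Overlap events count pawns to set the requested Open state, which Tick copies to IsOpen only while unlocked.
; Tick eases the door's relative rotation toward the open or closed target each frame.
; The construction script applies configurable meshes, optional flipping, and the initial open, closed or locked pose.
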(event OnComponentBeginOverlap(TriggerBox)
  (params (OtherActor :type Actor%20Object%20Reference) (OtherComp :type Primitive%20Component%20Object%20Reference) (OtherBodyIndex :type Integer) (bFromSweep :type Boolean) (SweepResult :type Hit%20Result%20Structure%20%28by%20ref%29))
  ;[1 1 1] Try to open the door.
  (Utilities|Casting|CastToPawn OtherActor)
  (bind _output_get (Variables|Internal|SetActorCount (+ (Variables|Internal|GetActorCount) 1)))
  (if (!= _output_get 0)
    (Variables|Door|SetOpen true)
    (else
      (Variables|Door|SetOpen false))))

(event OnComponentEndOverlap(TriggerBox)
  (params (OtherActor :type Actor%20Object%20Reference) (OtherComp :type Primitive%20Component%20Object%20Reference) (OtherBodyIndex :type Integer))
  ;[1 1 1] Try to close the door
  (Utilities|Casting|CastToPawn OtherActor)
  (bind _output_get (Variables|Internal|SetActorCount (- (Variables|Internal|GetActorCount) 1)))
  (if (== _output_get 0)
    (Variables|Door|SetOpen false)))

(event EventTick
  (params (DeltaSeconds :type Float%20%28single-precision%29))
  (bind _returnvalue (* DeltaSeconds 4.0))
  (bind _sm_door (Variables|Default|GetSM_Door))
  (bind _open (Variables|Door|GetOpen))
  (bind _relativerotation (Variables|/Script/Engine.SceneComponent|GetRelativeRotation _sm_door))
  (Utilities|FlowControl|Sequence
    (:then_0
      ;[1 1 1] Animate the Door
      (if (Variables|Internal|GetIsOpen)
        (Transformation|SetRelativeRotation _sm_door (Math|Interpolation|Ease "Linear" _returnvalue _relativerotation (Variables|Internal|GetTargetOpen) true) false)
        (else
          (Transformation|SetRelativeRotation _sm_door (Math|Interpolation|Ease "Linear" _returnvalue _relativerotation (Variables|Internal|GetTargetClosed) true) false))))
    (:then_1
      ;[1 1 1] Check if the open state changed and adjust accordingly
      (if (and (not (Variables|Door|GetLock)) (Math|Boolean|NotEqual(Boolean) _open (Variables|Internal|GetIsOpen)))
        (Variables|Internal|SetIsOpen _open)))))

(fn ConstructionScript
  (bind _sm_door (Variables|Default|GetSM_Door))
  (bind _targetclosed (Variables|Internal|GetTargetClosed))
  (Utilities|FlowControl|Sequence
    (:then_0
      ;[0.1 0.1 0.1] Adjust used StaticMesh
      (Components|StaticMesh|SetStaticMesh (Variables|Default|GetSM_DoorFrame) (Variables|Construction|GetDoor%20Frame%20SM))
      (Components|StaticMesh|SetStaticMesh (Variables|Default|GetSM_Door) (Variables|Construction|GetDoor%20SM)))
    (:then_1
      ;[0.1 0.1 0.1] Create the door flipped?
      (if (Variables|Construction|GetFlip)
        (|SetNewTargets
          (:exec
            (Transformation|SetRelativeLocation (Variables|Default|GetDoor%20Rotation%20Origin) "10.000000,-45.000000, 0" false)))))
    (:then_2
      ;[0.1 0.1 0.1] Should the Door be locked initially? (Will close the door!)
      (if (Variables|Door|GetLock)
        (Transformation|SetRelativeRotation _sm_door _targetclosed false)
        (else
          ;;[0.2 0.2 0.2] Should the Door spawn in an open position?
          (if (Variables|Door|GetOpen)
            (Transformation|SetRelativeRotation _sm_door (Variables|Internal|GetTargetOpen) false)
            (else
              (Transformation|SetRelativeRotation _sm_door _targetclosed false))))))))